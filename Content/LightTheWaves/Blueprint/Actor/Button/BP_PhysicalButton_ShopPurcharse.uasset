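; A physical shop button that buys its assigned PurchasableDefinition when activated.
; Activation calls TryPurchase on the CB shop subsystem and plays a 2D purchase sound on success.
; The construction script labels the button with the upgrade name and cost.
; Highlight enables custom depth on the button body and passes RemoveHighlight to a zero-time timer, which Unreal does not schedule.
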(event Custom|RemoveHighlight
  (Rendering|SetRenderCustomDepth (Variables|Default|GetButtonBody) false))

(event EventBeginPlay
  (|CallParentFunction) ; This node is disabled and will not be called.\nDrag off pins to build functionality.
)

(event Collision|EventActorBeginOverlap
  (params (OtherActor :type Actor%20Object%20Reference))
  (|CallParentFunction OtherActor) ; This node is disabled and will not be called.\nDrag off pins to build functionality.
)

(event EventTick
  (params (DeltaSeconds :type Float%20%28single-precision%29))
  (|CallParentFunction DeltaSeconds) ; This node is disabled and will not be called.\nDrag off pins to build functionality.
)

(event EventOnButtonActivated
  (bind _returnvalue (Class|CBShopSubsystem|TryPurchase (Subsystems|GetCBShopSubsystem) (Variables|Default|GetPurchasable%20Definition)))
  (if (.bwassuccessful _returnvalue)
    (Audio|PlaySound2D "/Game/Audio/Sounds/MetaSounds/MS_ItemPurcharse.MS_ItemPurcharse" 1.0 1.0 0.0 0 0)))

(event EventHighlight
  (params (Duration :type Float%20%28double-precision%29))
  (Utilities|Time|SetTimerbyEvent (delegate Custom|RemoveHighlight) 0.0)
  (Rendering|SetRenderCustomDepth (Variables|Default|GetButtonBody) true))

(fn ConstructionScript
  (bind _purchasable_definition (Variables|Default|GetPurchasable%20Definition))
  (|CallParentFunction)
  (Rendering|Components|TextRender|SetText (Variables|Default|GetTextRender) (Utilities|Text|ToText(String) (Utilities|String|Append (Utilities|String|ToString(Name) (Variables|/Script/LightTheWaves.CBPurchasableDefinition|GetUpgradeName _purchasable_definition)) "(" (Utilities|String|ToString(Integer) (Variables|/Script/LightTheWaves.CBPurchasableDefinition|GetCost _purchasable_definition)) "$)"))))