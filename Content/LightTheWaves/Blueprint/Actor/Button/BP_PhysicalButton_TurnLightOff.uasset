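; Physical button actor that toggles a referenced light on and off when activated.
; A FlipFlop alternates between TurnOn and TurnOff on that light, starting with TurnOn despite the TurnLightOff asset name, and does nothing if the reference is invalid.
; A Highlight event enables custom depth rendering on the button body and sets a timer to remove it after the given duration.
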(event Custom|RemoveHighlight
  (Rendering|SetRenderCustomDepth (Variables|Default|GetButtonBody) false))

(event EventHighlight
  (params (Duration :type Float%20%28double-precision%29))
  (Utilities|Time|SetTimerbyEvent (delegate Custom|RemoveHighlight) Duration)
  (Rendering|SetRenderCustomDepth (Variables|Default|GetButtonBody) true))

(event EventOnButtonActivated
  (Utilities|IsValid (Variables|Default|GetLight)
    (:Is%20Valid
      (Utilities|FlowControl|FlipFlop
        (:A
          (Default|Turnon (Variables|Default|GetLight)))
        (:B
          (Default|TurnOff (Variables|Default|GetLight) true))))))

(fn ConstructionScript)