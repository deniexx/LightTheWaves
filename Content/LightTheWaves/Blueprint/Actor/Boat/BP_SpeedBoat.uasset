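; Speed boat actor that varies its hull look and flashes red when hit by debris.
; On BeginPlay it randomly picks a blue or default body material and binds to its debris-hit event.
; A hit creates dynamic instances of the mesh materials, then a Timeline blends their Colour parameter between white and red.
; The Timeline reverses or replays whenever it finishes, so the flash ping-pongs indefinitely.
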(event Custom|OnBoatHitByDebris_Event
  (for (_array_element _array_index) (Rendering|Material|GetMaterials (Variables|Default|GetBoatMesh))
    (bind _returnvalue (Rendering|Material|CreateDynamicMaterialInstance (Variables|Default|GetBoatMesh) _array_index _array_element "None" :!class /Script/Engine.PrimitiveComponent))
    (Utilities|Array|AddUnique (Variables|Default|GetMaterials) _returnvalue))
  (bind (_direction _alpha) (Timeline|Timeline Play)
    (:Update
      (for _array_element_2 (Variables|Default|GetMaterials)
        (Rendering|Material|SetVectorParameterValue _array_element_2 "Colour" (Math|Color|Lerp(LinearColor) "(R=1.000000,G=1.000000,B=1.000000,A=1.000000)" "(R=1.000000,G=0.000000,B=0.000000,A=1.000000)" _alpha) :!class /Script/Engine.MaterialInstanceDynamic)))
    (:Finished
      (switch Utilities|FlowControl|Switch|SwitchonETimelineDirection _direction
        (:Forward
          (Timeline|Timeline Reverse))
        (:Backward
          (Timeline|Timeline Play))))))

(event EventBeginPlay
  (|CallParentFunction)
  (EventDispatchers|BindEventtoOnBoatHitbyDebris (delegate Custom|OnBoatHitByDebris_Event))
  (Rendering|Material|SetMaterial (Variables|Default|GetBoatMesh) 0 (select (Math|Random|RandomBool) "/Game/LightTheWaves/Meshes/Boats/SpeedBoat/MI_SpeedBoat_BodyBlue.MI_SpeedBoat_BodyBlue" "/Game/LightTheWaves/Meshes/Boats/SpeedBoat/MI_SpeedBoat_Body.MI_SpeedBoat_Body")))

(fn ConstructionScript)