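; BP_AmmoLever is a lever actor that prompts an ammo chute to check for reloading when pulled.
; Activation and deactivation events toggle an IsActivated flag, and activation also calls ReloadCheck on the referenced AmmoChute.
; A timed Highlight event enables custom depth rendering on the lever, then a timer event switches it off after the given duration.
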(event Custom|RemoveHighlight
  (Rendering|SetRenderCustomDepth (Variables|Default|GetLever) false))

(event Collision|EventActorBeginOverlap
  (params (OtherActor :type Actor%20Object%20Reference))
  (|CallParentFunction OtherActor) ; This node is disabled and will not be called.\nDrag off pins to build functionality.
)

(event EventTick
  (params (DeltaSeconds :type Float%20%28single-precision%29))
  (|CallParentFunction DeltaSeconds) ; This node is disabled and will not be called.\nDrag off pins to build functionality.
)

(event EventOnLeverActivated
  (Variables|Default|SetIsActivated true)
  (Default|ReloadCheck (Variables|Default|GetAmmoChute)))

(event EventOnLeverDeActivated
  (Variables|Default|SetIsActivated false))

(event EventHighlight
  (params (Duration :type Float%20%28double-precision%29) (Infinite :type Boolean))
  (Rendering|SetRenderCustomDepth (Variables|Default|GetLever) true)
  (Utilities|Time|SetTimerbyEvent (delegate Custom|RemoveHighlight) Duration))

(event EventBeginPlay
  (|CallParentFunction) ; This node is disabled and will not be called.\nDrag off pins to build functionality.
)

(fn ConstructionScript
  (|CallParentFunction))