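; VR joystick-style lever that steers a LightActor across X and Y within set bounds.
; While a hook overlaps it, Tick aims the lever using the hook and body positions, then converts pitch and roll beyond a small deadzone into movement, with speed depending on whether the light is on.
; Grab and release play right-hand haptics, and release eases the lever back to its initial rotation.
; A timed highlight uses custom depth.
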(event Custom|RemoveHighlight
  (Rendering|SetRenderCustomDepth (Variables|Default|GetLever) false))

(event EventOnHookOverlapEnd
  (params (OverlapComponent :type Primitive%20Component%20Object%20Reference))
  (bind _lever (Variables|Default|GetLever))
  (Variables|Default|SetUpdateLight false)
  (Variables|Default|SetOverlap%20Component 0)
  (Physics|SetSimulatePhysics _lever false)
  (Class|PlayerController|PlayHapticEffect (Game|GetPlayerController 0) "/Game/VRTemplate/Haptics/GrabHapticEffect.GrabHapticEffect" "Right" 1.0 false)
  (Components|MoveComponentTo _lever (Variables|/Script/Engine.SceneComponent|GetRelativeLocation _lever) (Variables|Default|GetLevelInitialRotation) false false 0.2 true))

(event EventOnHookOverlapBegin
  (params (OverlapComponent :type Primitive%20Component%20Object%20Reference))
  (bind _lever (Variables|Default|GetLever))
  (Variables|Default|SetOverlap%20Component OverlapComponent)
  (Variables|Default|SetUpdateLight true)
  (Physics|SetSimulatePhysics _lever true)
  (Class|PlayerController|PlayHapticEffect (Game|GetPlayerController 0) "/Game/VRTemplate/Haptics/GrabHapticEffect.GrabHapticEffect" "Right" 1.0 false)
  (Components|MoveComponentTo _lever (Variables|/Script/Engine.SceneComponent|GetRelativeLocation _lever) (Variables|Default|GetLevelInitialRotation) false false 0.2 true) ; enters at Stop
)

(event EventTick
  (params (DeltaSeconds :type Float%20%28single-precision%29))
  (bind _lightactor (Variables|Default|GetLightActor))
  (bind _upperlightbounds (Variables|Default|GetUpperLightBounds))
  (bind _lowerlightbounds (Variables|Default|GetLowerLightBounds))
  (bind _lightspeed (Variables|Default|GetLightSpeed))
  (bind _lightactor_2 (Variables|Default|GetLightActor))
  (bind _lightspeedmultiplier (Variables|Default|GetLightSpeedMultiplier))
  (bind _lever (Variables|Default|GetLever))
  (bind _lever_2 (Variables|Default|GetLever))
  (bind _returnvalue (Transformation|GetActorLocation _lightactor))
  (bind _returnvalue_2 (* _lightspeed _lightspeedmultiplier))
  (bind _relativerotation (Variables|/Script/Engine.SceneComponent|GetRelativeRotation _lever_2))
  (bind _relativerotation_2 (Variables|/Script/Engine.SceneComponent|GetRelativeRotation _lever))
  (bind _lighton_ (Variables|/Game/LightTheWaves/Blueprint/Actor/Light/BP_Light.BP_Light_C|GetLightOn? _lightactor_2))
  (bind _returnvalue_3 (Math|Float|SelectFloat _lightspeed _returnvalue_2 _lighton_))
  (if (Variables|Default|GetUpdateLight)
    (Variables|Default|SetDelta%20Seconds DeltaSeconds)
    (Utilities|IsValid (Variables|Default|GetLightActor)
      (:Is%20Valid
        (Utilities|IsValid (Variables|Default|GetOverlap%20Component)
          (:Is%20Valid
            (Transformation|SetRelativeRotation (Variables|Default|GetLever) (Math|Rotator|FindLookatRotation (Transformation|GetWorldLocation (Variables|Default|GetOverlap%20Component)) (Transformation|GetWorldLocation (Variables|Default|GetBody))) false true)
            (if (or (> (Math|Float|Absolute(Float) (.roll _relativerotation)) 3.0) (> (Math|Float|Absolute(Float) (.pitch _relativerotation)) 3.0))
              (Transformation|SetActorLocation _lightactor (Math|Vector|MakeVector (Math|Float|Clamp(Float) (+ (.x _returnvalue) (* (* (/ (.pitch _relativerotation_2) 45.0) _returnvalue_3 (Variables|Default|GetDelta%20Seconds)) -1.0)) (.x _lowerlightbounds) (.x _upperlightbounds)) (Math|Float|Clamp(Float) (+ (.y _returnvalue) (* (/ (.roll _relativerotation_2) 45.0) _returnvalue_3 (Variables|Default|GetDelta%20Seconds))) (.y _lowerlightbounds) (.y _upperlightbounds)) (.z _returnvalue)) false false))))))))

(event EventBeginPlay
  (|CallParentFunction)
  (Physics|SetSimulatePhysics (Variables|Default|GetLever) false)
  (Variables|Default|SetLevelInitialRotation (Transformation|GetWorldRotation (Variables|Default|GetLever))))

(event EventHighlight
  (params (Duration :type Float%20%28double-precision%29))
  (Utilities|Time|SetTimerbyEvent (delegate Custom|RemoveHighlight) Duration)
  (Rendering|SetRenderCustomDepth (Variables|Default|GetLever) true))

(fn ConstructionScript)