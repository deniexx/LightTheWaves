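; BP_LightControl is a physical joystick-style lever that steers an assigned light actor horizontally.
; While a hook overlaps, the lever simulates physics and a magnetic force pulls it toward the hook component each tick.
; Lever pitch and roll beyond a small dead zone drive the light's X and Y movement, scaled by speed and clamped to bounds.
; When the overlap ends, physics stops and MoveComponentTo eases the lever back toward its saved initial rotation.
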(event EventOnHookOverlapEnd
  (params (OverlapComponent :type Primitive%20Component%20Object%20Reference))
  (bind _lever (Variables|Default|GetLever))
  (Variables|Default|SetUpdateLight false)
  (Variables|Default|SetOverlap%20Component 0)
  (Physics|SetSimulatePhysics _lever false)
  (Components|MoveComponentTo _lever (Variables|/Script/Engine.SceneComponent|GetRelativeLocation _lever) (Variables|Default|GetLevelInitialRotation) false false 0.2 true))

(event EventOnHookOverlapBegin
  (params (OverlapComponent :type Primitive%20Component%20Object%20Reference))
  (bind _lever (Variables|Default|GetLever))
  (Variables|Default|SetOverlap%20Component OverlapComponent)
  (Variables|Default|SetUpdateLight true)
  (Physics|SetSimulatePhysics _lever true)
  (Components|MoveComponentTo _lever (Variables|/Script/Engine.SceneComponent|GetRelativeLocation _lever) (Variables|Default|GetLevelInitialRotation) false false 0.2 true) ; enters at Stop
)

(event EventTick
  (params (DeltaSeconds :type Float%20%28single-precision%29))
  (bind _lightactor (Variables|Default|GetLightActor))
  (bind _upperlightbounds (Variables|Default|GetUpperLightBounds))
  (bind _lowerlightbounds (Variables|Default|GetLowerLightBounds))
  (bind _lever (Variables|Default|GetLever))
  (bind _lever_2 (Variables|Default|GetLever))
  (bind _returnvalue (Transformation|GetActorLocation _lightactor))
  (bind _relativerotation (Variables|/Script/Engine.SceneComponent|GetRelativeRotation _lever_2))
  (bind _relativerotation_2 (Variables|/Script/Engine.SceneComponent|GetRelativeRotation _lever))
  (if (Variables|Default|GetUpdateLight)
    (Variables|Default|SetDelta%20Seconds DeltaSeconds)
    (Utilities|IsValid (Variables|Default|GetLightActor)
      (:Is%20Valid
        (Utilities|IsValid (Variables|Default|GetOverlap%20Component)
          (:Is%20Valid
            (Physics|AddForce (Variables|Default|GetLever) (* (Math|Vector|Normalize (- (Transformation|GetWorldLocation (Variables|Default|GetOverlap%20Component)) (Transformation|GetWorldLocation (Variables|Default|GetLever)))) (Variables|Default|GetLightMagneticForce)) "None" true)
            (if (or (> (Math|Float|Absolute(Float) (.roll _relativerotation)) 3.0) (> (Math|Float|Absolute(Float) (.pitch _relativerotation)) 3.0))
              (Transformation|SetActorLocation _lightactor (Math|Vector|MakeVector (Math|Float|Clamp(Float) (+ (.x _returnvalue) (* (* (/ (.pitch _relativerotation_2) 45.0) (Variables|Default|GetLightSpeed) (Variables|Default|GetDelta%20Seconds)) -1.0)) (.x _lowerlightbounds) (.x _upperlightbounds)) (Math|Float|Clamp(Float) (+ (.y _returnvalue) (* (/ (.roll _relativerotation_2) 45.0) (Variables|Default|GetLightSpeed) (Variables|Default|GetDelta%20Seconds))) (.y _lowerlightbounds) (.y _upperlightbounds)) (.z _returnvalue)) false false))))))))

(event EventBeginPlay
  (|CallParentFunction)
  (Physics|SetSimulatePhysics (Variables|Default|GetLever) false)
  (Variables|Default|SetLevelInitialRotation (Transformation|GetWorldRotation (Variables|Default|GetLever))))

(fn ConstructionScript)