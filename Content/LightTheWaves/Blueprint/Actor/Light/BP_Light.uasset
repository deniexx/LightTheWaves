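; BP_Light is a guiding light actor that can be switched on and off and notifies actors entering its sphere.
; A dynamic material dims or brightens the mesh as sphere query collision toggles, starting off on BeginPlay.
; Sphere overlaps send focus begin and end messages to actors implementing CBLightInteractor.
; TurnOff acts instantly or after a timer, which TurnOn cancels.
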(event OnComponentBeginOverlap(Sphere)
  (params (OverlappedComponent :type Primitive%20Component%20Object%20Reference) (OtherActor :type Actor%20Object%20Reference) (OtherComp :type Primitive%20Component%20Object%20Reference) (OtherBodyIndex :type Integer) (bFromSweep :type Boolean) (SweepResult :type Hit%20Result%20Structure%20%28by%20ref%29))
  (Utilities|IsValid OtherActor
    (:Is%20Valid
      (if (Utilities|DoesObjectImplementInterface OtherActor "/Script/LightTheWaves.CBLightInteractor")
        (Class|CBLightInteractor|OnLightFocused(Message) OtherActor (Variables|Default|GetSphere))))))

(event OnComponentEndOverlap(Sphere)
  (params (OverlappedComponent :type Primitive%20Component%20Object%20Reference) (OtherActor :type Actor%20Object%20Reference) (OtherComp :type Primitive%20Component%20Object%20Reference) (OtherBodyIndex :type Integer))
  (Utilities|IsValid OtherActor
    (:Is%20Valid
      (if (Utilities|DoesObjectImplementInterface OtherActor "/Script/LightTheWaves.CBLightInteractor")
        (Class|CBLightInteractor|OnLightFocusEnd(Message) OtherActor)))))

(event Custom|TurnOn
  (bind _turnofftimerhandle (Variables|Default|GetTurnOffTimerHandle))
  (if (Utilities|Time|IsValidTimerHandle _turnofftimerhandle)
    (Utilities|Time|ClearandInvalidateTimerbyHandle _turnofftimerhandle))
  (Collision|SetCollisionEnabled (Variables|Default|GetSphere) "QueryOnly")
  (Rendering|Material|SetScalarParameterValue (Variables|Default|GetDynamicMaterial) "Opacity" 0.3 :!class /Script/Engine.MaterialInstanceDynamic))

(event Custom|TurnOff
  (params (Instant :type Boolean))
  (if Instant
    (CallFunction|TurnLightOffTimerElapsed)
    (else
      (bind _returnvalue (Utilities|Time|SetTimerbyEvent (delegate Custom|TurnLightOffTimer_Elapsed) (Variables|Default|GetLightTurnOffTimerDuration)))
      (Variables|Default|SetTurnOffTimerHandle _returnvalue))))

(event Custom|TurnLightOffTimer_Elapsed
  (Collision|SetCollisionEnabled (Variables|Default|GetSphere) "NoCollision")
  (Rendering|Material|SetScalarParameterValue (Variables|Default|GetDynamicMaterial) "Opacity" 0.05 :!class /Script/Engine.MaterialInstanceDynamic))

(event EventBeginPlay
  (bind _returnvalue (Rendering|Material|CreateDynamicMaterialInstance (Variables|Default|GetStaticMesh) 0 "/Game/Materials/Transparency/MI_GuidingLight.MI_GuidingLight" "None" :!class /Script/Engine.PrimitiveComponent))
  (Variables|Default|SetDynamicMaterial _returnvalue)
  (CallFunction|TurnOff true))

(event Collision|EventActorBeginOverlap
  (params (OtherActor :type Actor%20Object%20Reference)))

(event EventTick
  (params (DeltaSeconds :type Float%20%28single-precision%29)))

(fn ConstructionScript)