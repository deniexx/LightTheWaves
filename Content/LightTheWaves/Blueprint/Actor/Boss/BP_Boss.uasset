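; Boss actor that runs a looping timed attack and is destroyed when its TakeDamage function drains Health to near zero.
; Each attack chains three timelines: a turn to a random left or right angle, a roll-offset swing, then a return toward zero rotation.
; Timeline alphas feed RInterpTo as DeltaTime to drive the motion.
; The hit is only a debug print, with no collision check or damage dealt.
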(event Custom|Attack
  (Variables|Default|SetLeftRotation? (Math|Random|RandomBool))
  (bind _alpha (Timeline|RotateLR PlayFromStart)
    (:Update
      (Transformation|SetActorRotation (Math|Interpolation|RInterpTo "0, 0, 0" (Math|Rotator|SelectRotator "-10.000000,0.000000,0.000000" "10.000000,0.000000,0.000000" (Variables|Default|GetLeftRotation?)) _alpha 1.0)))
    (:Finished
      (Variables|Default|SetCurrent (Transformation|GetActorRotation))
      (bind _alpha_2 (Timeline|AttackTL PlayFromStart)
        (:Update
          (Transformation|SetActorRotation (Math|Interpolation|RInterpTo (Variables|Default|GetCurrent) (Math|Rotator|MakeRotator (+ (.roll (Variables|Default|GetCurrent)) 3e+01) (.pitch (Variables|Default|GetCurrent)) (.yaw (Variables|Default|GetCurrent))) _alpha_2 1.0)))
        (:Finished
          (Development|PrintString "Player Hit" true true "(R=1.000000,G=0.040901,B=0.000000,A=1.000000)" 1.0)
          (Variables|Default|SetCurrent (Transformation|GetActorRotation))
          (bind _alpha_3 (Timeline|ReturnTL PlayFromStart)
            (:Update
              (Transformation|SetActorRotation (Math|Interpolation|RInterpTo (Variables|Default|GetCurrent) "0, 0, 0" _alpha_3 1.0)))))))))

(event EventBeginPlay
  (Utilities|Time|SetTimerbyEvent (delegate Custom|Attack) 3.0 true))

(fn ConstructionScript)

(fn TakeDamage
  (params (Damage :type Float%20%28double-precision%29))
  (bind _output_get (Variables|Default|SetHealth (- (Variables|Default|GetHealth) Damage)))
  (if (<= (Math|Float|Clamp(Float) _output_get 0.0 1.2e+02) 0.1)
    (Actor|DestroyActor)
    (else
      (return))))