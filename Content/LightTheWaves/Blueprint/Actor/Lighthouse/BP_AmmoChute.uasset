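; Ammo chute actor in the lighthouse that triggers a reload on a gun or hand actor placed in it.
; Its capsule overlap events track an actor implementing CBGunInterface, storing it as the overlapping hand with a flag.
; The ReloadCheck event, with no caller in this graph, sends ReloadMessage to that actor when the flag is set and the AmmoLever is activated.
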(event OnComponentEndOverlap(Capsule)
  (params (OverlappedComponent :type Primitive%20Component%20Object%20Reference) (OtherActor :type Actor%20Object%20Reference) (OtherComp :type Primitive%20Component%20Object%20Reference) (OtherBodyIndex :type Integer))
  (if (Collision|IsOverlappingActor OtherActor (Variables|Default|GetOverlappingHand) :!class /Script/Engine.Actor)
    (Variables|Default|SetOverlappingHand 0)
    (Variables|Default|SetIsHandOverlap false)))

(event OnComponentBeginOverlap(Capsule)
  (params (OverlappedComponent :type Primitive%20Component%20Object%20Reference) (OtherActor :type Actor%20Object%20Reference) (OtherComp :type Primitive%20Component%20Object%20Reference) (OtherBodyIndex :type Integer) (bFromSweep :type Boolean) (SweepResult :type Hit%20Result%20Structure%20%28by%20ref%29))
  (if (Utilities|DoesObjectImplementInterface OtherActor "/Script/LightTheWaves.CBGunInterface")
    (Variables|Default|SetOverlappingHand OtherActor)
    (Variables|Default|SetIsHandOverlap true)))

(event Custom|ReloadCheck
  (if (Variables|Default|GetIsHandOverlap)
    (if (Variables|/Game/LightTheWaves/Blueprint/Actor/Lever/BP_AmmoLever.BP_AmmoLever_C|GetIsActivated (Variables|Default|GetAmmoLever))
      (Class|CBGunInterface|Reload(Message) (Variables|Default|GetOverlappingHand)))))

(event EventBeginPlay)

(event Collision|EventActorBeginOverlap
  (params (OtherActor :type Actor%20Object%20Reference)))

(event EventTick
  (params (DeltaSeconds :type Float%20%28single-precision%29)))

(fn ConstructionScript)