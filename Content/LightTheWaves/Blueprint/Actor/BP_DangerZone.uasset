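; BP_DangerZone is a placeable zone actor that notifies a CBBoat when it enters a monster zone.
; An overlap on ActivationBox calls MonsterZoneStateUpdate on the boat with an entrance state, and no exit is handled here.
; The construction script rebuilds InstancedPath, laying copies of PlacedMesh along a spline, spaced by mesh X extent plus an offset and rotated to follow the curve.
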(event OnComponentBeginOverlap(ActivationBox)
  (params (OverlappedComponent :type Primitive%20Component%20Object%20Reference) (OtherActor :type Actor%20Object%20Reference) (OtherComp :type Primitive%20Component%20Object%20Reference) (OtherBodyIndex :type Integer) (bFromSweep :type Boolean) (SweepResult :type Hit%20Result%20Structure%20%28by%20ref%29))
  (bind _ascbboat (Utilities|Casting|CastToCBBoat OtherActor))
  (Class|CBBoat|MonsterZoneStateUpdate _ascbboat (Variables|Default|GetEnterance?)))

(fn ConstructionScript
  (bind _placedmesh (Variables|Default|GetPlacedMesh))
  (bind _splinecomponent (Variables|Default|GetSplineComponent))
  (bind _returnvalue (StaticMesh|GetBoundingBox _placedmesh))
  (bind (_min _max) (Utilities|Struct|BreakBox _returnvalue))
  (Components|StaticMesh|SetStaticMesh (Variables|Default|GetInstancedPath) (Variables|Default|GetPlacedMesh))
  (Components|InstancedStaticMesh|ClearInstances (Variables|Default|GetInstancedPath))
  (bind _output_get (Variables|Default|SetSpacing (+ (.X (Class|KismetMathLibrary|BreakVector3f (- _max _min))) (Variables|Default|GetOffset))))
  (bind _output_get_2 (Variables|Default|SetNumberOfInstances (Math|Float|Floor (/ (Spline|GetSplineLength (Variables|Default|GetSplineComponent)) _output_get))))
  (for _index (range 0 _output_get_2)
    (Components|InstancedStaticMesh|AddInstance (Variables|Default|GetInstancedPath) (Math|Transform|MakeTransform (Spline|GetLocationatDistanceAlongSpline _splinecomponent (* _index (Variables|Default|GetSpacing)) "Local") (Spline|GetRotationatDistanceAlongSpline _splinecomponent (* _index (Variables|Default|GetSpacing)) "Local")) false)))