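; BP_Debris is a hazard actor that damages destroyable objects that touch it.
; When its sphere begins overlapping an actor implementing the CBDestroyableObject interface, it sends TakeDamageMessage with itself as instigator, a Debris type and its DebrisDamage amount.
; Highlight and UnHighlight events toggle custom depth rendering on its three floater components.
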(event OnComponentBeginOverlap(Sphere)
  (params (OverlappedComponent :type Primitive%20Component%20Object%20Reference) (OtherActor :type Actor%20Object%20Reference) (OtherComp :type Primitive%20Component%20Object%20Reference) (OtherBodyIndex :type Integer) (bFromSweep :type Boolean) (SweepResult :type Hit%20Result%20Structure%20%28by%20ref%29))
  (if (Utilities|DoesObjectImplementInterface OtherActor "/Script/LightTheWaves.CBDestroyableObject")
    (Class|CBDestroyableObject|TakeDamage(Message) OtherActor self "Debris" (Variables|Default|GetDebrisDamage))))

(event EventUnHighlight
  (Rendering|SetRenderCustomDepth (Variables|Default|GetFloater1) false))

(event EventHighlight
  (params (Duration :type Float%20%28double-precision%29) (Infinite :type Boolean))
  (Rendering|SetRenderCustomDepth (Variables|Default|GetFloater1) true))

(fn ConstructionScript)