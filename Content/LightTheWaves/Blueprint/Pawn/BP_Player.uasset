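; VR player pawn with a pull-cord projectile launcher that fires when the right hand pulls the handle past ShootDistance.
; Overlapping the handle box makes it follow the hand, resizing the cable and ramping haptics on both controllers.
; Each tick, a predicted projectile path feeds a Niagara trail and, in mortar mode, a distant landing marker.
; Firing or leaving the box hides the visuals and slides the handle back.
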(event OnComponentBeginOverlap(Box)
  (params (OverlappedComponent :type Primitive%20Component%20Object%20Reference) (OtherActor :type Actor%20Object%20Reference) (OtherComp :type Primitive%20Component%20Object%20Reference) (OtherBodyIndex :type Integer) (bFromSweep :type Boolean) (SweepResult :type Hit%20Result%20Structure%20%28by%20ref%29))
  (CallFunction|BeginOverlapPH OtherComp))

(event OnComponentEndOverlap(Box)
  (params (OverlappedComponent :type Primitive%20Component%20Object%20Reference) (OtherActor :type Actor%20Object%20Reference) (OtherComp :type Primitive%20Component%20Object%20Reference) (OtherBodyIndex :type Integer))
  (CallFunction|EndOverlapPH OtherComp))

(event Custom|EndOverlapPH
  (params (OtherComp :type Primitive%20Component%20Object%20Reference))
  (if (== OtherComp (Variables|Default|GetRightHandOverlapBox))
    (Variables|Default|SetUpdatingHandleRoot? false)
    (Collision|SetCollisionEnabled (Variables|Default|GetBox) "NoCollision")
    (Rendering|SetVisibility (Variables|Default|GetCable) false false)
    (Rendering|SetVisibility (Variables|Default|GetShotPath) false false)
    (Rendering|SetVisibility (Variables|Default|GetShotLocation) false false)
    (Audio|PlaySoundatLocation (Variables|Default|GetPullCordSound) (Transformation|GetWorldLocation (Variables|Default|GetShootReference)) "0, 0, 0" 1.0 1.0 0.0 0 0 0 0)
    (Components|MoveComponentTo (Variables|Default|GetHandleRoot) "60.000000,0.000000,10.000000" "0, 0, 0" false false 0.2 false)
    (Collision|SetCollisionEnabled (Variables|Default|GetBox) "QueryOnly")))

(event Custom|BeginOverlapPH
  (params (OtherComp :type Primitive%20Component%20Object%20Reference))
  (if (== OtherComp (Variables|Default|GetRightHandOverlapBox))
    (Variables|Default|SetUpdatingHandleRoot? true)
    (Rendering|SetVisibility (Variables|Default|GetCable) true false)
    (Rendering|SetVisibility (Variables|Default|GetShotPath) true false)
    (Components|MoveComponentTo (Variables|Default|GetHandleRoot) "60.000000,0.000000,10.000000" "0, 0, 0" false false 0.2 false) ; enters at Stop
  ))

(event Collision|EventActorBeginOverlap
  (params (OtherActor :type Actor%20Object%20Reference)))

(event EventTick
  (params (DeltaSeconds :type Float%20%28single-precision%29))
  (bind _returnvalue (Game|GetPlayerController 0))
  (bind _shootdistance (Variables|Default|GetShootDistance))
  (bind _handleroot (Variables|Default|GetHandleRoot))
  (bind _shootreference (Variables|Default|GetShootReference))
  (bind _relativelocation (Variables|/Script/Engine.SceneComponent|GetRelativeLocation _shootreference))
  (bind _relativelocation_2 (Variables|/Script/Engine.SceneComponent|GetRelativeLocation _handleroot))
  (bind _returnvalue_2 (Math|Vector|Distance(Vector) _relativelocation_2 _relativelocation))
  (bind _returnvalue_3 (/ _returnvalue_2 _shootdistance))
  (if (Variables|Default|GetUpdatingHandleRoot?)
    (Transformation|SetWorldLocationAndRotation (Variables|Default|GetHandleRoot) (Transformation|GetWorldLocation (Variables|Default|GetHookRef)) (Transformation|GetWorldRotation (Variables|Default|GetHandRight)) false false)
    (Variables|/Script/CableComponent.CableComponent|SetCableLength (Variables|Default|GetCable) (Math|Vector|Distance(Vector) (Variables|/Script/Engine.SceneComponent|GetRelativeLocation (Variables|Default|GetCableAttachEnd)) _relativelocation))
    (bind (_outhit _outpathpositions _outlasttracedestination) (Class|GameplayStatics|BlueprintPredictProjectilePathbyTraceChannel (Transformation|GetWorldLocation (Variables|Default|GetShootLocation)) (Class|CBPawn|GetLaunchVelocityforProjectile) true 32.0 (select (Variables|Default|GetbMortarMode) "ECC_GameTraceChannel3" "ECC_GameTraceChannel2") false (Utilities|Array|MakeArray self) "None" 0.0 15.0 (Class|CBPawn|GetProjectileLifeSpan)))
    (Class|NiagaraDataInterfaceArrayFunctionLibrary|SetNiagaraArrayVector (Variables|Default|GetShotPath) "PointArray" _outpathpositions)
    (if (> (Math|Vector|Distance(Vector) _outlasttracedestination (Transformation|GetActorLocation)) 1e+03)
      (Rendering|SetVisibility (Variables|Default|GetShotLocation) (Variables|Default|GetbMortarMode) false)
      (Transformation|SetWorldLocation (Variables|Default|GetShotLocation) (Math|Vector|MakeVector (.X (Class|KismetMathLibrary|BreakVector3f _outlasttracedestination)) (.Y (Class|KismetMathLibrary|BreakVector3f _outlasttracedestination)) 5e+01) false false)
      (else
        (Rendering|SetVisibility (Variables|Default|GetShotLocation) false false)
        (Niagara|SetNiagaraVariable(Float) (Variables|Default|GetShotLocation) "Radius" (Class|CBPawn|GetProjectileAreaOfEffect))))
    (if (> _returnvalue_2 _shootdistance)
      (Class|CBPawn|Shoot)
      (CallFunction|EndOverlapPH (Variables|Default|GetRightHandOverlapBox))
      (Class|PlayerController|PlayHapticEffect _returnvalue "/Game/VRTemplate/Haptics/PistolFireHapticEffect.PistolFireHapticEffect" "Left" 1e+01 false)
      (Class|PlayerController|PlayHapticEffect _returnvalue "/Game/VRTemplate/Haptics/PistolFireHapticEffect.PistolFireHapticEffect" "Right" 5.0 false)
      (else
        (Class|PlayerController|PlayHapticEffect _returnvalue "/Game/VRTemplate/Haptics/PistolFireHapticEffect.PistolFireHapticEffect" "Left" (* _returnvalue_3 3.0) false)
        (Class|PlayerController|PlayHapticEffect _returnvalue "/Game/VRTemplate/Haptics/PistolFireHapticEffect.PistolFireHapticEffect" "Right" (* _returnvalue_3 3.6) false)))))

(fn ConstructionScript)