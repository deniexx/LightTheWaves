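; Game mode for a lighthouse defense game, running the scripted tutorial, wave and recess feedback, shop purchase messages and the lose screen.
; The tutorial chains delays, boat and ammo delegates and boss events, pairing notifications and highlights with voice lines played at the computer.
; Activity state changes announce waves, trigger a one-time shop hint and manage a spawned end-recess button.
; Shop purchases select notifications by gameplay tag.
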(event Custom|OnActivityStateUpdated_Event
  (params (ActivityStateUpdatedData :type Activity%20State%20Updated%20Data%20Structure))
  (Utilities|FlowControl|Sequence
    (:then_0
      (switch Utilities|FlowControl|Switch|SwitchonEGameActivity (.oldactivity ActivityStateUpdatedData)
        (:Wave
          (switch Utilities|FlowControl|Switch|SwitchonEActivityFinishedState (.activityfinishedstate ActivityStateUpdatedData)
            (:Successful
              (Class|CBBlueprintFunctionLibrary|SendNotification "Wave Ended!" 3.0)
              (Utilities|FlowControl|DoOnce false
                (:Completed
                  (|Execute (Utilities|Struct|MakeTutorialDisplayParams 0 "/Game/LightTheWaves/Blueprint/Actor/WidgetActors/BP_TutorialActor.BP_TutorialActor_C" "Shop for Items behind you!" "0.000000,90.000000,0.000000" "0.000000,0.000000,40.000000" (Variables|Default|GetTutorial%20Display%20Params%20Text%20Color) 20 "/Engine/EditorSounds/GamePreview/EndSimulate_Cue.EndSimulate_Cue" 8.0))
                  (bind _outactors (Actor|GetAllActorsOfClass "/Game/LightTheWaves/Blueprint/Actor/Button/BP_PhysicalButton_ShopPurcharse.BP_PhysicalButton_ShopPurcharse_C"))
                  (for _array_element _outactors
                    (Class|BPIHighlightableActor|Highlight(Message) _array_element 1e+01)
                    (Audio|PlaySoundatLocation "/Game/Audio/Sounds/VA/VA_EndWave.VA_EndWave" (Transformation|GetActorLocation (Variables|Default|GetComputer)) "0, 0, 0" 1.0 1.0 0.0 0 0 0 0)))))))))
    (:then_1
      (switch Utilities|FlowControl|Switch|SwitchonEGameActivity (.newactivity ActivityStateUpdatedData)
        (:Wave
          (if (Utilities|Enum|Equal(Enum) (.oldactivity ActivityStateUpdatedData) "Recess")
            (Class|CBBlueprintFunctionLibrary|SendNotification "Wave Starting!" 3.0)
            (bind _recessbutton (Variables|Default|GetRecessButton)
              (:then
                (Actor|DestroyActor _recessbutton))
              (:else))))
        (:Recess
          (bind _returnvalue (Game|SpawnActorfromClass "/Game/LightTheWaves/Blueprint/Actor/Button/BP_PhysicalButton_EndRecess.BP_PhysicalButton_EndRecess_C" (Math|Transform|MakeTransform "-603.000000,7929.000000,4014.000000" "0.000000,-50.000000,90.000000" "0.100000,0.100000,0.100000") "AlwaysSpawn" "MultiplyWithRoot" 0 0))
          (Variables|Default|SetRecessButton _returnvalue))))))

(event Custom|OnBoatReachedport
  (bind _ascbpawn (Utilities|Casting|CastToCBPawn (Game|Player|GetPlayerPawn 0)))
  (EventDispatchers|BindEventtoOnAmmoUpdated _ascbpawn (delegate Custom|AmmoUpdated))
  (bind _returnvalue (Actor|GetActorOfClass "/Game/LightTheWaves/Blueprint/Actor/Lighthouse/BP_AmmoChute.BP_AmmoChute_C"))
  (Class|BPIHighlightableActor|Highlight(Message) (Variables|/Game/LightTheWaves/Blueprint/Actor/Lighthouse/BP_AmmoChute.BP_AmmoChute_C|GetRegularChute _returnvalue) 1e+01)
  (Class|BPIHighlightableActor|Highlight(Message) (Variables|/Game/LightTheWaves/Blueprint/Actor/Lighthouse/BP_AmmoChute.BP_AmmoChute_C|GetAmmoLever (Variables|/Game/LightTheWaves/Blueprint/Actor/Lighthouse/BP_AmmoChute.BP_AmmoChute_C|GetRegularChute _returnvalue)) 1e+01)
  (Class|CBBlueprintFunctionLibrary|SendNotification "Insert the cannon in the highlighted ammo chute and pull the lever to reload" 1e+01)
  (Audio|PlaySoundatLocation "/Game/Audio/Sounds/VA/VA_AmmoChute.VA_AmmoChute" (Transformation|GetActorLocation (Variables|Default|GetComputer)) "0, 0, 0" 1.0 1.0 0.0 0 0 0 0))

(event Custom|SpawnBoatTut
  (bind _returnvalue (Class|CBGameMode|SpawnBoat 0 "/Game/LightTheWaves/Blueprint/Actor/Boat/BP_SpeedBoat.BP_SpeedBoat_C"))
  (bind _ascbboat (Utilities|Casting|CastToCBBoat _returnvalue))
  (EventDispatchers|AssignOnBoatDead _ascbboat (delegate Custom|OnBoatDead))
  (Utilities|FlowControl|Delay (Math|Random|RandomFloatinRange 25.0 3e+01))
  (Class|CBGameMode|SpawnMonster))

(event Custom|OnBoatDead
  (params (DestroyingObject :type EDestroyingObject%20Enum :default "Debris"))
  (if (Utilities|Enum|Equal(Enum) DestroyingObject "Port")
    (CallFunction|OnBoatReachedport)
    (else
      (Class|CBBlueprintFunctionLibrary|SendNotification "When a boat dies, you lose some reputation. Lose too much and you'll be fired." 1e+01)
      (Utilities|FlowControl|Delay (Math|Random|RandomFloatinRange 3.0 5.0))
      (CallFunction|SpawnBoatTut)
      (Audio|PlaySoundatLocation "/Game/Audio/Sounds/VA/VA_WhenaBoatSinks.VA_WhenaBoatSinks" (Transformation|GetActorLocation (Variables|Default|GetComputer)) "0, 0, 0" 1.0 1.0 0.0 0 0 0 0))))

(event Custom|AmmoUpdated
  (params (NewAmmoCount :type Integer) (MaxAmmo :type Integer))
  (if (> NewAmmoCount 0)
    (EventDispatchers|UnbindEventfromOnAmmoUpdated (stale Custom|OnBoatReachedport _ascbpawn) (delegate Custom|AmmoUpdated))
    (Utilities|FlowControl|Delay 5.0)
    (Class|CBGameMode|SpawnBoss)
    (Class|CBBlueprintFunctionLibrary|SendNotification "Shoot the beast!" 1e+01)
    (Audio|PlaySoundatLocation "/Game/Audio/Sounds/VA/VA_UglyBeast.VA_UglyBeast" (Transformation|GetActorLocation (Variables|Default|GetComputer)) "0, 0, 0" 1.0 1.0 0.0 0 0 0 0)))

(event Custom|OnShopItemBought_Event
  (params (Purchasable :type CB%20Purchasable%20Definition%20Object%20Reference) (Amount :type Integer))
  (bind _returnvalue (> Amount 1))
  (Utilities|FlowControl|Sequence
    (:then_0
      (|SwitchGameplayTag (Variables|/Script/LightTheWaves.CBPurchasableDefinition|GetIdentityTag Purchasable)
        (:Purchasable.AmmoUpgrade
          (Variables|Default|SetNotification "Ammo Capacity Upgraded!"))
        (:Purchasable.MortarAmmo
          (Variables|Default|SetNotification (Utilities|String|SelectString "Mortar Ammo Added!" "Use the second chute to load mortar ammo. It is used to destroy hazards in the water." _returnvalue))
          (if (not _returnvalue)
            (bind _returnvalue_2 (Actor|GetActorOfClass "/Game/LightTheWaves/Blueprint/Actor/Lighthouse/BP_AmmoChute.BP_AmmoChute_C"))
            (Class|BPIHighlightableActor|Highlight(Message) (Variables|/Game/LightTheWaves/Blueprint/Actor/Lighthouse/BP_AmmoChute.BP_AmmoChute_C|GetMortarChute _returnvalue_2) 1e+01)
            (Class|BPIHighlightableActor|Highlight(Message) (Variables|/Game/LightTheWaves/Blueprint/Actor/Lighthouse/BP_AmmoChute.BP_AmmoChute_C|GetAmmoLever2 _returnvalue_2) 1e+01)
            (Audio|PlaySoundatLocation "/Game/Audio/Sounds/VA/VA_MortarAmmo.VA_MortarAmmo" (Transformation|GetActorLocation (Variables|Default|GetComputer)) "0, 0, 0" 1.0 1.0 0.0 0 0 0 0)))
        (:Purchasable.ReputationUpgrade
          (Variables|Default|SetNotification "Maximum reputation has been Increased!"))))
    (:then_1
      (Class|CBBlueprintFunctionLibrary|SendNotification (Variables|Default|GetNotification) (Math|Float|SelectFloat 5.0 1e+01 _returnvalue)))))

(event EventBeginPlay
  (|CallParentFunction)
  (EventDispatchers|AssignOnActivityStateUpdated (delegate Custom|OnActivityStateUpdated_Event))
  (bind _returnvalue (Class|CBBlueprintFunctionLibrary|GetShopSubsystem))
  (EventDispatchers|AssignOnShopItemBought _returnvalue (delegate Custom|OnShopItemBought_Event))
  (bind _returnvalue_2 (Actor|GetActorOfClass "/Game/LightTheWaves/Blueprint/Actor/WidgetActors/BP_Computer.BP_Computer_C"))
  (Variables|Default|SetComputer _returnvalue_2))

(event EventPlayTutorial
  (Utilities|FlowControl|Delay 2.0)
  (Audio|PlaySoundatLocation "/Game/Audio/Sounds/VA/VA_Intro.VA_Intro" (Transformation|GetActorLocation (Variables|Default|GetComputer)) "0, 0, 0" 1.0 1.0 0.0 0 0 0 0)
  (Utilities|FlowControl|Delay 6.0)
  (CallFunction|SpawnBoatTut)
  (Utilities|FlowControl|Delay 4.0)
  (Class|CBBlueprintFunctionLibrary|SendNotification "Move the light with the highlighted object. If the light is close to the boats they will follow it." 1e+01)
  (bind _returnvalue (Actor|GetActorOfClass "/Game/LightTheWaves/Blueprint/Actor/Light/BP_LightControl.BP_LightControl_C"))
  (Class|BPIHighlightableActor|Highlight(Message) _returnvalue 1e+01)
  (Audio|PlaySoundatLocation "/Game/Audio/Sounds/VA/VA_Joystick.VA_Joystick" (Transformation|GetActorLocation (Variables|Default|GetComputer)) "0, 0, 0" 1.0 1.0 0.0 0 0 0 0)
  (Utilities|FlowControl|Delay 1e+01)
  (Class|CBBlueprintFunctionLibrary|SendNotification "You can press the highlighted button to turn the light on/off." 1e+01)
  (bind _returnvalue_2 (Actor|GetActorOfClass "/Game/LightTheWaves/Blueprint/Actor/Button/BP_PhysicalButton_TurnLightOff.BP_PhysicalButton_TurnLightOff_C"))
  (Class|BPIHighlightableActor|Highlight(Message) _returnvalue_2 1e+01)
  (Audio|PlaySoundatLocation "/Game/Audio/Sounds/VA/VA_LightButton.VA_LightButton" (Transformation|GetActorLocation (Variables|Default|GetComputer)) "0, 0, 0" 1.0 1.0 0.0 0 0 0 0)
  (Utilities|FlowControl|Delay 8.0)
  (Audio|PlaySoundatLocation "/Game/Audio/Sounds/VA/VA_BoatsCantSee.VA_BoatsCantSee" (Transformation|GetActorLocation (Variables|Default|GetComputer)) "0, 0, 0" 1.0 1.0 0.0 0 0 0 0)
  (Class|CBGameMode|SpawnMonster))

(event EventOnGameFinished
  (params (Data :type Game%20Lost%20Data%20Structure%20%28by%20ref%29))
  (bind _returnvalue (Game|SpawnActorfromClass "/Game/LightTheWaves/Blueprint/Game/BP_LoseScreen.BP_LoseScreen_C" (Math|Transform|MakeTransform "-468.000000,7701.000000,3967.000000" "0.000000,90.000000,0.000000" "1.000000,1.000000,1.000000") "Undefined" "MultiplyWithRoot" 0 0))
  (Default|SetLoseReason _returnvalue (Utilities|Text|ToText(String) (.losereason Data))))

(event EventOnBossKilledTutorial
  (Utilities|FlowControl|DoOnce false
    (:Completed
      (Class|CBWaveDirector|StartWaveGameplay(Message) self)
      (Class|CBBlueprintFunctionLibrary|SendNotification "Wave starting! Good Luck!" 7.0)
      (Audio|PlaySoundatLocation "/Game/Audio/Sounds/VA/VA_NowYoureReady.VA_NowYoureReady" (Transformation|GetActorLocation (Variables|Default|GetComputer)) "0, 0, 0" 1.0 1.0 0.0 0 0 0 0)
      (Utilities|FlowControl|Delay 4.0)
      (Audio|PlaySoundatLocation "/Game/Audio/Sounds/VA/VA_InfoPosters.VA_InfoPosters" (Transformation|GetActorLocation (Variables|Default|GetComputer)) "0, 0, 0" 1.0 1.0 0.0 0 0 0 0))))

(fn ConstructionScript)