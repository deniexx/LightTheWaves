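; BP_LoseScreen is an in-world lose screen that shows why the player lost and their points, and restarts the level.
; On BeginPlay a timeline moves the Letter component upward in relative space.
; SetLoseReason writes the given reason and the PlayerState's points message into the WBP_LoseMessage hosted by its widget component.
; Any overlap with the Box reopens the current level by name.
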(event OnComponentBeginOverlap(Box)
  (params (OverlappedComponent :type Primitive%20Component%20Object%20Reference) (OtherActor :type Actor%20Object%20Reference) (OtherComp :type Primitive%20Component%20Object%20Reference) (OtherBodyIndex :type Integer) (bFromSweep :type Boolean) (SweepResult :type Hit%20Result%20Structure%20%28by%20ref%29))
  (bind _returnvalue (Game|GetCurrentLevelName true))
  (Game|OpenLevel(byName) (Utilities|String|StringToName _returnvalue)))

(event Custom|SetLoseReason
  (params (LoseText :type Text))
  (bind _aswbp_lose_message (Utilities|Casting|CastToWBP_LoseMessage (UserInterface|GetWidget (Variables|Default|GetWidget))))
  (Rendering|Components|TextRender|SetText (Variables|/Game/LightTheWaves/Blueprint/Game/WBP_LoseMessage.WBP_LoseMessage_C|GetTextBlock_ReasonText _aswbp_lose_message) LoseText)
  (bind _returnvalue (Class|CBPlayerInterface|GetPoints(Message) (Game|GetPlayerState 0)))
  (Rendering|Components|TextRender|SetText (Variables|/Game/LightTheWaves/Blueprint/Game/WBP_LoseMessage.WBP_LoseMessage_C|GetTextBlock_Points _aswbp_lose_message) (Utilities|Text|ToText(String) (Utilities|String|Append "Points: " (Utilities|String|ToString(Integer) _returnvalue)))))

(event EventBeginPlay
  (bind _alpha (Timeline|MoveLetterTL Play)
    (:Update
      (Transformation|SetRelativeLocation (Variables|Default|GetLetter) (Math|Vector|Lerp(Vector) "0, 0, 0" "0.000000,0.000000,110.000000" _alpha) false false))))

(fn ConstructionScript)